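; Assignment actor that builds a small vertex-colored procedural mesh at BeginPlay, after a short delay.
; It creates one mesh section from the Pos vertices and two triangles taken from the Ind index vectors.
; Six vertex colors come from two Cols entries, three each, rescaled from 0-255 to 0-1.
; M_Vertex is then applied, and the mesh is scaled up with a negative X that mirrors it.
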(event `self.ReceiveBeginPlay`
  (bind _proceduralmesh (`self.ProceduralMesh`))
  (bind _cols (`self.cols`))
  (bind _ind (`self.ind`))
  (bind (_output_x _output_y _output_z) (break `IntVector` (`|GetArrayItem` _ind 1)))
  (bind (_output_x_2 _output_y_2 _output_z_2) (break `IntVector` (`|GetArrayItem` _ind)))
  (bind (_returnvalue_x _returnvalue_y _returnvalue_z) (`KismetMathLibrary.BreakVector` (/ (`|GetArrayItem` _cols 3) 255)))
  (bind (_returnvalue_x_2 _returnvalue_y_2 _returnvalue_z_2) (`KismetMathLibrary.BreakVector` (/ (`|GetArrayItem` _cols) 255)))
  (bind _returnvalue (`KismetMathLibrary.MakeColor` _returnvalue_x_2 _returnvalue_y_2 _returnvalue_z_2))
  (bind _returnvalue_2 (`KismetMathLibrary.MakeColor` _returnvalue_x _returnvalue_y _returnvalue_z))
  (`KismetSystemLibrary.Delay` 0.2)
  (`ProceduralMeshComponent.CreateMeshSection_LinearColor` :`self` _proceduralmesh :`Vertices` (`self.pos`) :`Triangles` (`|MakeArray` _output_x_2 _output_y_2 _output_z_2 _output_x _output_y _output_z) :`VertexColors` (`|MakeArray` _returnvalue _returnvalue _returnvalue _returnvalue_2 _returnvalue_2 _returnvalue_2))
  (`PrimitiveComponent.SetMaterial` _proceduralmesh 0 "/Game/Assignment_1/M_Vertex.M_Vertex")
  (`SceneComponent.SetRelativeScale3D` _proceduralmesh (-10.0 10.0 10.0)))

(fn `UserConstructionScript`)